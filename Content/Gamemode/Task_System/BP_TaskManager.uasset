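; Task manager that tracks player tasks from a data table and changes the ghost's chase rate as they are completed.
; UpdateTaskAvailability rebuilds the Available and Locked lists by checking each row's TaskID and UnlockID against Completed.
; CompleteTask matches an ObjectID to an available task, records it, passes its appeasement value to the ghost and refreshes the lists.
; GetCurrentTaskList supplies display text padded with blanks to five entries; BeginPlay creates the task widget.
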(event EventBeginPlay
  (bind _returnvalue (UserInterface|CreateWidget "/Game/UI/TaskWidget.TaskWidget_C" 0 self))
  (UserInterface|Viewport|AddtoViewport _returnvalue 0)
  (CallFunction|UpdateTaskAvailability))

(fn ConstructionScript)

(fn GetCurrentTaskList
  (for _array_element (Variables|Default|Getavailable)
    (bind _returnvalue (Utilities|GetDataTableRow "/Game/Gamemode/Task_System/TaskTable.TaskTable" _array_element)
      (:then
        (Utilities|Array|Add (LocalVariables|Gettask_text_array) (.display_text (Utilities|Struct|BreakTask _returnvalue))))))
  ;[1 1 1] checks if there are up to 5 tasks in  the task list
  (if (< (Utilities|Array|Length (LocalVariables|Gettask_text_array)) 5)
    ;[1 1 1] adds blank tasks to the UI if there are less than 5 tasks
    (for _index (range 0 (- 5 (Utilities|Array|Length (LocalVariables|Gettask_text_array))))
      (Utilities|Array|Add (LocalVariables|Gettask_text_array) "")))
  (return (LocalVariables|Gettask_text_array)))

(fn UpdateTaskAvailability
  ;[1 1 1] empties the locked and available arrays to refresh them
  (Utilities|Array|Clear (Variables|Default|Getlocked))
  (Utilities|Array|Clear (Variables|Default|Getavailable))
  (bind _outrownames (DataTable|GetDataTableRowNames "/Game/Gamemode/Task_System/TaskTable.TaskTable"))
  (for _array_element _outrownames
    (bind _returnvalue (Utilities|GetDataTableRow "/Game/Gamemode/Task_System/TaskTable.TaskTable" _array_element)
      (:then
        ;[1 1 1] checks if a task was completed already. If it isn't completed but the task unlock ID is completed, add to the available task list
        (for _array_element_2 (Variables|Default|Getcompleted)
          (bind _returnvalue_2 (Utilities|GetDataTableRow "/Game/Gamemode/Task_System/TaskTable.TaskTable" _array_element_2)
            (:then
              (if (Utilities|Name|Equal(Name) (.task_ID (Utilities|Struct|BreakTask _returnvalue_2)) (.task_ID (Utilities|Struct|BreakTask _returnvalue)))
                (LocalVariables|Setin_completed true)
                (elif (Utilities|Name|Equal(Name) (.task_ID (Utilities|Struct|BreakTask _returnvalue_2)) (.unlock_ID (Utilities|Struct|BreakTask _returnvalue)))
                  (Utilities|Array|Add (Variables|Default|Getavailable) ""))))))
        (if (LocalVariables|Getin_completed)
          _
          (else
            ;[1 1 1] add tasks with no unlock requirements to the task list
            (if (Utilities|Name|Equal(Name) (.unlock_ID (Utilities|Struct|BreakTask _returnvalue)) "000")
              (Utilities|Array|Add (Variables|Default|Getavailable) (.task_ID (Utilities|Struct|BreakTask _returnvalue)))
              (else
                ;[1 1 1] add any remaining tasks to the locked list
                (Utilities|Array|Add (Variables|Default|Getlocked) (.task_ID (Utilities|Struct|BreakTask _returnvalue)))))))
        (LocalVariables|Setin_completed false))))
  (CallFunction|GetCurrentTaskList))

(fn CompleteTask
  (params (object_ID :type Name))
  (bind _outrownames (DataTable|GetDataTableRowNames "/Game/Gamemode/Task_System/TaskTable.TaskTable"))
  (for _array_element _outrownames
    (bind _returnvalue (Utilities|GetDataTableRow "/Game/Gamemode/Task_System/TaskTable.TaskTable" _array_element)
      (:then
        ;[1 1 1] checks if task has been completed
        (if (Utilities|Name|Equal(Name) (.object_ID (Utilities|Struct|BreakTask _returnvalue)) object_ID)
          ;[1 1 1] checks if task was actually available to be completed
          (for _array_element_2 (Variables|Default|Getavailable)
            (if (Utilities|Name|Equal(Name) _array_element_2 (.task_ID (Utilities|Struct|BreakTask _returnvalue)))
              (LocalVariables|Setavailable_to_complete true)))
          (if (LocalVariables|Getavailable_to_complete)
            (Utilities|Array|Add (Variables|Default|Getcompleted) (.task_ID (Utilities|Struct|BreakTask _returnvalue)))
            (Default|ChangeChaseRate (Variables|Default|Getghost_reference) (.appeasement_value (Utilities|Struct|BreakTask _returnvalue))))))))
  (CallFunction|UpdateTaskAvailability))