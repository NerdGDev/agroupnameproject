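; BP_Ghost1 is an enemy ghost that trails the player and periodically rattles chains.
; Each Tick it lerps by delta time toward a point Speed units behind the player controller, rotating to face that point.
; Speed acts as follow distance, which ChangeChaseRate reduces by the given modifier.
; A delay loop from BeginPlay keeps resetting the looping rattle timer to random intervals, playing a sound and debug print.
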(event EventBeginPlay
  (bind _returnvalue (Math|Random|RandomFloatinRange 4.0 25.0))
  (Utilities|Time|SetTimerbyFunctionName 0 "rattle" _returnvalue true :!label _label)
  (Utilities|FlowControl|RetriggerableDelay _returnvalue)
  (goto _label))

(event Collision|EventActorBeginOverlap
  (params (OtherActor :type Actor%20Object%20Reference)))

(event EventTick
  (params (DeltaSeconds :type Float%20%28single-precision%29))
  (CallFunction|ChasePlayer DeltaSeconds))

(fn ConstructionScript)

(fn PickupObject)

(fn ChasePlayer
  (params (tick :type Float%20%28single-precision%29))
  (bind _returnvalue (Game|GetPlayerController 0))
  (bind _speed (Variables|Default|Getspeed))
  (bind _returnvalue_2 (Transformation|GetActorForwardVector _returnvalue))
  (bind _returnvalue_3 (Transformation|GetActorLocation _returnvalue))
  (bind _returnvalue_4 (* _returnvalue_2 -1))
  (bind _returnvalue_5 (* _returnvalue_4 _speed))
  (bind _returnvalue_6 (+ _returnvalue_5 _returnvalue_3))
  (Transformation|SetActorLocationAndRotation (Math|Vector|Lerp(Vector) (Transformation|GetActorLocation) _returnvalue_6 tick) (Math|Rotator|FindLookatRotation (Transformation|GetActorLocation) _returnvalue_6)))

(fn ChangeChaseRate
  (params (chase_modifier :type Integer))
  (Variables|Default|Setspeed (- (Variables|Default|Getspeed) chase_modifier)))

(fn Rattle
  (Audio|PlaySoundatLocation "/Game/Assets/Sound/SmallChainRattle_Cue.SmallChainRattle_Cue" (Transformation|GetActorLocation) "0, 0, 0" 1.0 1.0 0.0 0 0 0)
  (Development|PrintString "sound played"))