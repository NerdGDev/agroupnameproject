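; Interactable world object that registers with BP_Gamemode and can hurt players while flagged as thrown.
; On BeginPlay it hides the Cube, shows BaseMesh and adds itself to the gamemode's interactables.
; When it overlaps a non-ghost BP_PlayerCharacter while thrown, it deals damage equal to its Weight.
; The trailing Delay after damage drives nothing, and IsThrown is never changed here.
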(event EventBeginPlay
  (Rendering|SetVisibility (Variables|Default|GetCube) false false)
  (Rendering|SetVisibility (Variables|Default|GetBaseMesh) true false)
  (bind _asbp_gamemode (Utilities|Casting|CastToBP_Gamemode (Game|GetGameMode)))
  (Default|AddInteractable _asbp_gamemode self))

(event Collision|EventActorBeginOverlap
  (params (OtherActor :type Actor%20Object%20Reference))
  (if (Variables|Default|Getis_thrown)
    (bind _asbp_player_character (Utilities|Casting|CastToBP_PlayerCharacter OtherActor))
    (if (not (Variables|/Game/Gamemode/ThirdPerson_Character/BP_PlayerCharacter.BP_PlayerCharacter_C|Getis_ghost _asbp_player_character))
      (Default|TakeDamage _asbp_player_character (Variables|Default|Getweight))
      (Utilities|FlowControl|Delay 5.0))))

(fn ConstructionScript)